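; Player character Blueprint that lets the player interact with nearby objects implementing the Interactable interface.
; BeginPlay creates a hidden interaction hint widget, which a Sphere overlap shows for interactable actors and hides once none remain inside.
; Tick polls for an E key press and sends InteractMessage to the first interactable actor overlapping the sphere, so only one responds per press.
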(event OnComponentBeginOverlap(Sphere)
  (params (OverlappedComponent :type Primitive%20Component%20Object%20Reference) (OtherActor :type Actor%20Object%20Reference) (OtherComp :type Primitive%20Component%20Object%20Reference) (OtherBodyIndex :type Integer) (bFromSweep :type Boolean) (SweepResult :type Hit%20Result%20Structure%20%28by%20ref%29))
  ;[1 1 1 0.038] show hint
  (if (Utilities|DoesObjectImplementInterface OtherActor "/Script/Horror.Interactable")
    (Widget|SetVisibility (Variables|Default|GetInteractHint) "Visible")))

(event OnComponentEndOverlap(Sphere)
  (params (OverlappedComponent :type Primitive%20Component%20Object%20Reference) (OtherActor :type Actor%20Object%20Reference) (OtherComp :type Primitive%20Component%20Object%20Reference) (OtherBodyIndex :type Integer))
  ;[1 1 1 0.092] hide hint
  (if (Utilities|DoesObjectImplementInterface OtherActor "/Script/Horror.Interactable")
    ;;[1 1 1] Checks if there are still interactive items nearby
    (if (not (Class|Utils|ContainsImplementation (Collision|GetOverlappingActors (Variables|Default|GetSphere) 0 :!class /Script/Engine.PrimitiveComponent) "/Script/Horror.Interactable"))
      (Widget|SetVisibility (Variables|Default|GetInteractHint) "Hidden"))))

(event EventTick
  (params (DeltaSeconds :type Float%20%28single-precision%29))
  ;[1 1 1 0.046] Interact
  ;;[1 1 1] interception of pressing the E button
  (if (Game|Player|WasInputKeyJustPressed (Game|GetPlayerController 0) "E")
    ;;[1 1 1] interaction with one interactive object, if there is one nearby
    (bind _array_element (Utilities|Array|ForEachLoopwithBreak (Collision|GetOverlappingActors (Variables|Default|GetSphere) 0 :!class /Script/Engine.PrimitiveComponent) :!label _label)
      (:LoopBody
        (if (Utilities|DoesObjectImplementInterface _array_element "/Script/Horror.Interactable")
          (Class|Interactable|Interact(Message) _array_element)
          (goto _label Break))))))

(event EventBeginPlay
  (Utilities|FlowControl|Sequence
    (:then_0
      (bind _returnvalue (UserInterface|CreateWidget "/Game/Blueprints/UI/WBP_InteractionHint.WBP_InteractionHint_C" (Game|GetPlayerController 0)))
      (bind _output_get (Variables|Default|SetInteractHint _returnvalue))
      (UserInterface|Viewport|AddtoViewport _output_get 0)
      (Widget|SetVisibility (Variables|Default|GetInteractHint) "Hidden"))))

(fn ConstructionScript)