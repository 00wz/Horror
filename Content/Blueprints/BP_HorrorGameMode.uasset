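; Game mode for a horror note-collecting game that keeps the enemy near the player and tracks win and loss.
; BeginPlay caches the player, enemy and all notes; each found note is removed, and an empty list triggers the win.
; Tick teleports an enemy that strays too far to a navmesh-projected point on a circle around the player, then restarts its behavior tree.
; Win and loss handlers only print messages.
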(event EventBeginPlay
  (bind _returnvalue (Actor|GetActorOfClass "/Game/Blueprints/BP_MainCharacter.BP_MainCharacter_C"))
  (Variables|Default|SetPlayer _returnvalue)
  (bind _returnvalue_2 (Actor|GetActorOfClass "/Game/Blueprints/BP_Enemy_.BP_Enemy__C"))
  (Variables|Default|SetEnemy _returnvalue_2)
  (bind _outactors (Actor|GetAllActorsOfClass "/Game/Blueprints/BP_Note.BP_Note_C"))
  (Variables|Default|SetNotes _outactors))

(event EventTick
  (params (DeltaSeconds :type Float%20%28single-precision%29))
  (CallFunction|EnemyDistanceCheck))

(fn ConstructionScript)

(fn GetPlayerActor
  (return (Variables|Default|GetPlayer)))

(fn GetMaxEnemyDestinationDistance
  (return (Variables|Default|GetMaxEnemyDestinationDistance)))

(fn GetSpawnPoint
  (bind _returnvalue (Math|Float|MakeLiteralFloat 5e+02))
  (bind _player (Variables|Default|GetPlayer))
  (bind _spawnenemydistance (Variables|Default|GetSpawnEnemyDistance))
  (bind _returnvalue_2 (Class|Utils|GetRandomVectoronCircle _spawnenemydistance))
  (bind _returnvalue_3 (Transformation|GetActorLocation _player))
  (bind _returnvalue_4 (+ _returnvalue_2 _returnvalue_3))
  (bind (_projectedlocation _returnvalue_5) (AI|Navigation|ProjectPointtoNavigation _returnvalue_4 0 0 (Math|Vector|MakeVector 0.0 0.0 _returnvalue)))
  (return _projectedlocation _returnvalue_5))

(fn EnemyDistanceCheck
  ;[1 1 1] Checking that the enemy is too far away
  (if (> (Class|KismetMathLibrary|VectorDistanceSquared (Transformation|GetActorLocation (Variables|Default|GetPlayer)) (Transformation|GetActorLocation (Variables|Default|GetEnemy))) (Math|Float|Square (Variables|Default|GetMaxEnemyDistance)))
    (bind (_spawnposition _result) (CallFunction|GetSpawnPoint))
    (if _result
      ;[1 1 1] it is necessary to teleport the enemy to a distance greater than its viewing radius, because artificial intelligence will break if the player remains in the field of view
      (CallFunction|TeleportEnemy _spawnposition))))

(fn TeleportEnemy
  (params (Positon :type Vector))
  (Transformation|SetActorLocation (Variables|Default|GetEnemy) Positon false true)
  (Default|RestartBehaviourTree (Variables|Default|GetEnemy)))

(fn OnFindingNote
  (params (Note :type BP%20Note%20Object%20Reference))
  (Utilities|Array|RemoveItem (Variables|Default|GetNotes) Note)
  ;[1 1 1] verifying that all notes have been collected
  (if (<= (Utilities|Array|Length (Variables|Default|GetNotes)) 0)
    (CallFunction|OnWinning)))

(fn OnWinning
  (Development|PrintString "Win!!!"))

(fn OnLosing
  (Development|PrintString "Losing!!!" true true "(R=1.000000,G=0.000000,B=0.018122,A=1.000000)"))