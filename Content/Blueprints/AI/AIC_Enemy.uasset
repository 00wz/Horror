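; AI controller for enemies that runs BT_Enemy and feeds it what perception detects about the player.
; Perception updates for the actor returned by BP_HorrorGameMode set the Player blackboard key while sensed and clear it when lost.
; On loss, it also stores the player's current location as LastPlayerPosition.
; SetSightRadius exposes runtime adjustment of the sight and lose-sight radii.
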(event OnTargetPerceptionUpdated(AIPerception)
  (params (Actor :type Actor%20Object%20Reference) (Stimulus :type AI%20Stimulus%20Structure))
  ;[1 1 1] Checking that the player has been detected
  (bind _asbp_horror_game_mode (Utilities|Casting|CastToBP_HorrorGameMode (Game|GetGameMode)))
  (if (== (Default|GetPlayerActor _asbp_horror_game_mode) Actor)
    (Utilities|FlowControl|Sequence
      (:then_0
        ;[1 1 1] if a player is lost, we set his last position
        (if (not (.bsuccessfullysensed Stimulus))
          (AI|Components|Blackboard|SetValueasVector (AI|GetBlackboard 0) (Utilities|Name|MakeLiteralName "LastPlayerPosition") (Transformation|GetActorLocation (Default|GetPlayerActor _asbp_horror_game_mode)))))
      (:then_1
        ;[1 1 1] set a link to the player or null if he is lost
        (AI|Components|Blackboard|SetValueasObject (AI|GetBlackboard 0) (Utilities|Name|MakeLiteralName "Player") (Utilities|SelectObject (Default|GetPlayerActor _asbp_horror_game_mode) 0 (.bsuccessfullysensed Stimulus)))))))

(event EventBeginPlay
  (AI|RunBehaviorTree "/Game/Blueprints/AI/BT_Enemy.BT_Enemy"))

(fn ConstructionScript)

(fn SetSightRadius
  (params (SightRadius :type Float%20%28single-precision%29) (LoseSightRadius :type Float%20%28single-precision%29))
  (Class|Utils|SetSightRadius (Variables|Default|GetAIPerception) SightRadius LoseSightRadius))